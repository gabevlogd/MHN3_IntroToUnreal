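; BP_TriggerBox is a trigger volume that reveals a set of target actors while something overlaps it.
; On BeginPlay it hides every actor in TargetActors.
; Its CollisionComponent begin overlap unhides them all and end overlap hides them again, with no filter on the overlapping actor or count of concurrent overlaps.
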(event OnComponentBeginOverlap(CollisionComponent)
  (params (OverlappedComponent :type Primitive%20Component%20Object%20Reference) (OtherActor :type Actor%20Object%20Reference) (OtherComp :type Primitive%20Component%20Object%20Reference) (OtherBodyIndex :type Integer) (bFromSweep :type Boolean) (SweepResult :type Hit%20Result%20Structure%20%28by%20ref%29))
  (for _array_element (Variables|Default|GetTargetActors)
    (Rendering|SetActorHiddenInGame _array_element false)))

(event OnComponentEndOverlap(CollisionComponent)
  (params (OverlappedComponent :type Primitive%20Component%20Object%20Reference) (OtherActor :type Actor%20Object%20Reference) (OtherComp :type Primitive%20Component%20Object%20Reference) (OtherBodyIndex :type Integer))
  (for _array_element (Variables|Default|GetTargetActors)
    (Rendering|SetActorHiddenInGame _array_element true)))

(event EventBeginPlay
  (for _array_element (Variables|Default|GetTargetActors)
    (Rendering|SetActorHiddenInGame _array_element true)))

(fn ConstructionScript)