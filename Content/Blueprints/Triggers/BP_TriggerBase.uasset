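; BP_TriggerBase is a trigger actor that turns the platform beneath it green when a Character overlaps it and restores the colour on player death.
; On BeginPlay it binds to the player character's death event and traces downward to find the platform.
; It creates a dynamic material on the hit component and caches the "Checker Colour 2" start colour.
; HighlightPlatform writes that parameter for both overlap and reset.
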(event OnComponentBeginOverlap(CollisionComponent)
  (params (OverlappedComponent :type Primitive%20Component%20Object%20Reference) (OtherActor :type Actor%20Object%20Reference) (OtherComp :type Primitive%20Component%20Object%20Reference) (OtherBodyIndex :type Integer) (bFromSweep :type Boolean) (SweepResult :type Hit%20Result%20Structure%20%28by%20ref%29))
  (Utilities|Casting|CastToCharacter OtherActor)
  (CallFunction|HighlightPlatform "(R=0.000000,G=1.000000,B=0.030458,A=1.000000)"))

(event Custom|OnPlayerDeath_Event
  (CallFunction|HighlightPlatform (Variables|Default|GetStartColor)))

(event EventBeginPlay
  (bind _returnvalue (Transformation|GetActorLocation))
  (bind _asbp_mixamo_character (Utilities|Casting|CastToBP_MixamoCharacter (Game|GetPlayerCharacter 0)))
  (EventDispatchers|BindEventtoOnPlayerDeath _asbp_mixamo_character (EventDispatchers|CreateEvent :!event Custom|OnPlayerDeath_Event))
  (bind _outhit (Collision|LineTraceForObjects _returnvalue (+ _returnvalue "0.000000,0.000000,-500.000000") (Utilities|Array|MakeArray "ObjectTypeQuery1" "ObjectTypeQuery2") false 0 "None"))
  (Utilities|IsValid (Rendering|Material|GetMaterial (.HitComponent (Collision|BreakHitResult _outhit)) 0)
    (:Is%20Valid
      (bind _returnvalue_2 (Rendering|Material|CreateDynamicMaterialInstance (.HitComponent (Collision|BreakHitResult _outhit)) 0 (Rendering|Material|GetMaterial (.HitComponent (Collision|BreakHitResult _outhit)) 0) "None" :!class /Script/Engine.PrimitiveComponent))
      (bind _output_get (Variables|Default|SetPlatformMaterial _returnvalue_2))
      (bind _returnvalue_3 (Rendering|Material|GetVectorParameterValue _output_get "Checker Colour 2" :!class /Script/Engine.MaterialInstanceDynamic))
      (Variables|Default|SetStartColor _returnvalue_3))))

(fn ConstructionScript)

(fn HighlightPlatform
  (params (Value :type Linear%20Color%20Structure))
  (Rendering|Material|SetVectorParameterValue (Variables|Default|GetPlatformMaterial) "Checker Colour 2" Value :!class /Script/Engine.MaterialInstanceDynamic))