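; Trigger volume that starts a set of moving platforms when a Character enters its collision component.
; Platforms are paused at BeginPlay and resumed on overlap by toggling tick on each one's InterpToMovement component.
; A DoOnce limits the camera shutter sound to the first overlap until the Reset event rearms it.
; It also binds a delegate to the player character's death event at BeginPlay.
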(event OnComponentBeginOverlap(CollisionComponent)
  (params (OverlappedComponent :type Primitive%20Component%20Object%20Reference) (OtherActor :type Actor%20Object%20Reference) (OtherComp :type Primitive%20Component%20Object%20Reference) (OtherBodyIndex :type Integer) (bFromSweep :type Boolean) (SweepResult :type Hit%20Result%20Structure%20%28by%20ref%29))
  (Utilities|Casting|CastToCharacter OtherActor)
  (CallFunction|EnablePlatforms true)
  (Utilities|FlowControl|DoOnce false
    (:Completed
      (Audio|PlaySound2D "/Engine/VREditor/Sounds/UI/Camera_Shutter.Camera_Shutter" 1.0 1.0 0.0 0 0))))

(event Custom|Reset
  (Utilities|FlowControl|DoOnce false) ; enters at Reset
)

(event EventBeginPlay
  (CallFunction|EnablePlatforms false)
  (bind _asbp_third_person_character (Utilities|Casting|CastToBP_ThirdPersonCharacter (Game|GetPlayerCharacter 0)))
  (EventDispatchers|BindEventtoOnPlayerDeath _asbp_third_person_character (EventDispatchers|CreateEvent :!event Custom|Reset)))

(fn ConstructionScript)

(fn EnablePlatforms
  (params (bEnabled :type Boolean))
  (for _array_element (Variables|Default|GetPlatforms)
    (Components|Tick|SetComponentTickEnabled (Variables|/Game/Blueprints/Platforms/BP_Platform.BP_Platform_C|GetInterpToMovement _array_element) bEnabled)))

(fn NewFunction0)