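; Trigger that erases a list of actors when a Character first overlaps it, restoring them on player death.
; Static mesh actors get a dynamic material whose Dissolve is timeline-driven; others are hidden without collision.
; Each actor also plays a sound and Niagara effect.
; The loop shares one timeline and current-actor variable, so only the last dissolve instance animates and the finish callback disables collision only on the last actor.
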(event OnComponentBeginOverlap(CollisionComponent)
  (params (OverlappedComponent :type Primitive%20Component%20Object%20Reference) (OtherActor :type Actor%20Object%20Reference) (OtherComp :type Primitive%20Component%20Object%20Reference) (OtherBodyIndex :type Integer) (bFromSweep :type Boolean) (SweepResult :type Hit%20Result%20Structure%20%28by%20ref%29))
  (Utilities|Casting|CastToCharacter OtherActor)
  (Utilities|FlowControl|DoOnce false
    (:Completed
      (for _array_element (Variables|Default|GetActors)
        (Variables|Default|SetCurrentActor _array_element)
        (Utilities|FlowControl|Sequence
          (:then_0
            (Utilities|IsValid (Actor|GetComponentbyClass (Variables|Default|GetCurrentActor) "/Script/Engine.StaticMeshComponent")
              (:Is%20Valid
                (bind _returnvalue (Rendering|Material|CreateDynamicMaterialInstance (Actor|GetComponentbyClass (Variables|Default|GetCurrentActor) "/Script/Engine.StaticMeshComponent") 0 (Rendering|Material|GetMaterial (Actor|GetComponentbyClass (Variables|Default|GetCurrentActor) "/Script/Engine.StaticMeshComponent") 0) "None" :!class /Script/Engine.PrimitiveComponent))
                (bind _newtrack_0 (Timeline|Timeline PlayFromStart)
                  (:Update
                    (Rendering|Material|SetScalarParameterValue _returnvalue "Dissolve" _newtrack_0 :!class /Script/Engine.MaterialInstanceDynamic))))
              (:Is%20Not%20Valid
                (Rendering|SetActorHiddenInGame (Variables|Default|GetCurrentActor) true)
                (Collision|SetActorEnableCollision (Variables|Default|GetCurrentActor) false))))
          (:then_1
            (Audio|PlaySoundatLocation "/Engine/EditorSounds/GamePreview/EjectFromPlayer.EjectFromPlayer" (Transformation|GetActorLocation (Variables|Default|GetCurrentActor)) "0, 0, 0" 1.0 1.0 0.0 0 0 0 0)
            (bind _returnvalue_2 (Niagara|SpawnSystematLocation "/Niagara/DefaultAssets/Templates/Systems/AttributeReaderTrails.AttributeReaderTrails" (Transformation|GetActorLocation (Variables|Default|GetCurrentActor)) "0, 0, 0" "1.000000,1.000000,1.000000" true true "AutoRelease"))
            (Variables|Default|SetVFX _returnvalue_2)))))))

(event Custom|OnTimelineFinished
  (Collision|SetActorEnableCollision (Variables|Default|GetCurrentActor) false))

(event Custom|Reset
  (Utilities|FlowControl|DoOnce false) ; enters at Reset
)

(event EventBeginPlay
  (|CallParentFunction)
  (Class|TimelineComponent|SetTimelineFinishedFunc (Variables|Default|GetTimeline) (EventDispatchers|CreateEvent :!event Custom|OnTimelineFinished)))

(event EventOnPlayerDeathEvent
  (|CallParentFunction)
  (CallFunction|Reset)
  (for _array_element (Variables|Default|GetActors)
    (bind _output_get (Variables|Default|SetCurrentActor _array_element))
    (Rendering|SetActorHiddenInGame _output_get false)
    (Collision|SetActorEnableCollision (Variables|Default|GetCurrentActor) true)
    (bind _vfx (Variables|Default|GetVFX)
      (:then
        (Components|Activation|SetActive _vfx false true))
      (:else
        _))
    (Utilities|IsValid (Actor|GetComponentbyClass (Variables|Default|GetCurrentActor) "/Script/Engine.StaticMeshComponent")
      (:Is%20Valid
        (bind _returnvalue (Rendering|Material|CreateDynamicMaterialInstance (Actor|GetComponentbyClass (Variables|Default|GetCurrentActor) "/Script/Engine.StaticMeshComponent") 0 (Rendering|Material|GetMaterial (Actor|GetComponentbyClass (Variables|Default|GetCurrentActor) "/Script/Engine.StaticMeshComponent") 0) "None" :!class /Script/Engine.PrimitiveComponent))
        (Rendering|Material|SetScalarParameterValue _returnvalue "Dissolve" 1.0 :!class /Script/Engine.MaterialInstanceDynamic)))))

(fn ConstructionScript)