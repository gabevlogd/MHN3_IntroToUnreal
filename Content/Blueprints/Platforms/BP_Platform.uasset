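; BP_Platform is a moving platform that follows control points through an InterpToMovement component, built in the construction script from a location array as relative positions.
; Enable and disable functions toggle that component's tick to run or freeze movement.
; At each reversal it freezes and starts a short one-shot timer.
; On player death, bound through the ThirdPersonCharacter's dispatcher, it freezes and clears that timer.
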(event OnInterptoReverse(InterpToMovement)
  (params (ImpactResult :type Hit%20Result%20Structure%20%28by%20ref%29) (Time :type Float%20%28single-precision%29))
  (CallFunction|DisablePlatform)
  (bind _returnvalue (Utilities|Time|SetTimerbyEvent (EventDispatchers|CreateEvent :!event EnablePlatform) 3.0))
  (Variables|Default|SetPlatformTimer _returnvalue))

(event Custom|OnPlayerDeath_Event
  (CallFunction|DisablePlatform)
  (Utilities|Time|ClearandInvalidateTimerbyHandle (Variables|Default|GetPlatformTimer)))

(event EventBeginPlay
  (bind _asbp_third_person_character (Utilities|Casting|CastToBP_ThirdPersonCharacter (Game|GetPlayerCharacter 0)))
  (EventDispatchers|BindEventtoOnPlayerDeath _asbp_third_person_character (EventDispatchers|CreateEvent :!event Custom|OnPlayerDeath_Event)))

(fn ConstructionScript
  (for _array_element (Variables|Default|GetControlPointLocations)
    (Utilities|Array|Add (Variables|/Script/Engine.InterpToMovementComponent|GetControlPoints (Variables|Default|GetInterpToMovement)) (Utilities|Struct|MakeInterpControlPoint _array_element true))))

(fn DisablePlatform
  (Components|Tick|SetComponentTickEnabled (Variables|Default|GetInterpToMovement) false))

(fn EnablePlatform
  (Components|Tick|SetComponentTickEnabled (Variables|Default|GetInterpToMovement) true))