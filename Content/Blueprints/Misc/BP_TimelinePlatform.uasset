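; BP_TimelinePlatform is an actor whose static mesh moves back and forth between a Start and End location.
; On BeginPlay it sets the timeline length from Duration, binds a finished callback and plays.
; Each update lerps the mesh's relative location by normalized playback position, without sweep, and records the direction.
; When finished, it waits a fixed delay, then uses that direction to play from start or reverse from end.
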(event Custom|OnFinished
  (Utilities|FlowControl|Delay 4.0)
  (if (Utilities|Enum|Equal(Enum) (Variables|Default|GetLastDirection) "Backward")
    (Components|Timeline|PlayfromStart (Variables|Default|GetTimeline))
    (else
      (Components|Timeline|ReversefromEnd (Variables|Default|GetTimeline)))))

(event EventBeginPlay
  (bind _timeline (Variables|Default|GetTimeline))
  (Components|Timeline|SetTimelineLength (Variables|Default|GetTimeline) (Variables|Default|GetDuration))
  (Class|TimelineComponent|SetTimelineFinishedFunc (Variables|Default|GetTimeline) (EventDispatchers|CreateEvent :!event Custom|OnFinished))
  (bind _direction (Timeline|Timeline Play)
    (:Update
      (Variables|Default|SetLastDirection _direction)
      (Transformation|SetRelativeLocation (Variables|Default|GetStaticMesh) (Math|Vector|Lerp(Vector) (Variables|Default|GetStart) (Variables|Default|GetEnd) (/ (Components|Timeline|GetPlaybackPosition _timeline) (Class|TimelineComponent|GetScaledTimelineLength _timeline))) false false))))

(fn ConstructionScript)