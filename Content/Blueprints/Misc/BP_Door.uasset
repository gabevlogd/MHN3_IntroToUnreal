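; BP_Door is an interactable door that players can swing open and closed.
; A box overlap binds to the BP_MixamoCharacter's OnInteract dispatcher and shows a text prompt, undoing both on exit.
; ToggleDoor plays or reverses a timeline based on its last recorded direction, allowing mid-swing reversal.
; The timeline lerps mesh rotation by normalized playback position, with its length set from DoorAnimDuration at BeginPlay.
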(event OnComponentBeginOverlap(Box)
  (params (OverlappedComponent :type Primitive%20Component%20Object%20Reference) (OtherActor :type Actor%20Object%20Reference) (OtherComp :type Primitive%20Component%20Object%20Reference) (OtherBodyIndex :type Integer) (bFromSweep :type Boolean) (SweepResult :type Hit%20Result%20Structure%20%28by%20ref%29))
  ;[1 1 1] Interaction logic
  (bind _asbp_mixamo_character (Utilities|Casting|CastToBP_MixamoCharacter OtherActor))
  (EventDispatchers|BindEventtoOnInteract _asbp_mixamo_character (EventDispatchers|CreateEvent :!event Custom|ToggleDoor))
  (CallFunction|Highlight))

(event OnComponentEndOverlap(Box)
  (params (OverlappedComponent :type Primitive%20Component%20Object%20Reference) (OtherActor :type Actor%20Object%20Reference) (OtherComp :type Primitive%20Component%20Object%20Reference) (OtherBodyIndex :type Integer))
  ;[1 1 1] Interaction logic
  (bind _asbp_mixamo_character (Utilities|Casting|CastToBP_MixamoCharacter OtherActor))
  (EventDispatchers|UnbindEventfromOnInteract _asbp_mixamo_character (EventDispatchers|CreateEvent :!event Custom|ToggleDoor))
  (CallFunction|Unhighlight))

(event Custom|ToggleDoor
  ;[1 1 1] Toggoling door logic
  (if (Utilities|Enum|Equal(Enum) (Variables|Default|GetLastDirection) "Forward")
    (Utilities|String|Reverse (Variables|Default|GetDoorAnimation))
    (else
      (Audio|Components|Audio|Play (Variables|Default|GetDoorAnimation)))))

(event EventBeginPlay
  (Components|Timeline|SetTimelineLength (Variables|Default|GetDoorAnimation) (Variables|Default|GetDoorAnimDuration))
  (CallFunction|Unhighlight))

(fn ConstructionScript)

(fn Highlight
  (Rendering|SetVisibility (Variables|Default|GetTextRender) true false))

(fn Unhighlight
  (Rendering|SetVisibility (Variables|Default|GetTextRender) false false))