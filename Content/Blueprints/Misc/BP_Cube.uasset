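; BP_Cube is a cube Blueprint with a path-movement component and a surface area calculation.
; Its construction script adds each ControlPoints entry to InterpToMovement as a relative control point.
; BeginPlay disables that component's tick, so the movement stays idle, and nothing here re-enables it.
; GetArea returns six times the square of Edge.
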(event EventBeginPlay
  (Components|Tick|SetComponentTickEnabled (Variables|Default|GetInterpToMovement) false))

(fn ConstructionScript
  (for _array_element (Variables|Default|GetControlPoints)
    (Utilities|Array|Add (Variables|/Script/Engine.InterpToMovementComponent|GetControlPoints (Variables|Default|GetInterpToMovement)) (Utilities|Struct|MakeInterpControlPoint _array_element true))))

(fn GetArea
  (return (* (Math|Float|Power (Variables|Default|GetEdge) 2.0) 6.0)))