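; BP_LightTrigger is a trigger actor that switches a set of linked lights on while a character is inside its collision component.
; The lights start off at BeginPlay, turn on at character begin overlap and turn off at end overlap.
; SetEnableLights loops over the Lights array and sets each intensity to the default value multiplied by the enable flag, rather than toggling visibility.
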(event OnComponentBeginOverlap(CollisionComponent)
  (params (OverlappedComponent :type Primitive%20Component%20Object%20Reference) (OtherActor :type Actor%20Object%20Reference) (OtherComp :type Primitive%20Component%20Object%20Reference) (OtherBodyIndex :type Integer) (bFromSweep :type Boolean) (SweepResult :type Hit%20Result%20Structure%20%28by%20ref%29))
  (Utilities|Casting|CastToCharacter OtherActor)
  (CallFunction|SetEnableLights true))

(event OnComponentEndOverlap(CollisionComponent)
  (params (OverlappedComponent :type Primitive%20Component%20Object%20Reference) (OtherActor :type Actor%20Object%20Reference) (OtherComp :type Primitive%20Component%20Object%20Reference) (OtherBodyIndex :type Integer))
  (Utilities|Casting|CastToCharacter OtherActor)
  (CallFunction|SetEnableLights false))

(event EventBeginPlay
  (CallFunction|SetEnableLights false))

(fn ConstructionScript)

(fn SetEnableLights
  (params (Enable :type Boolean))
  (for _array_element (Variables|Default|GetLights)
    (Rendering|Components|Light|SetIntensity (Variables|/Script/Engine.Light|GetLightComponent _array_element) (* (Variables|Default|GetDefalutLightIntensity) (Math|Conversions|ToFloat(Boolean) Enable)))))