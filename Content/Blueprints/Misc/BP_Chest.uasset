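; Interactable chest that the player opens once, swinging its lid and playing a sound and Niagara effect.
; Box overlap shows or hides a text prompt and binds or unbinds the third-person character's OnInteract event while the chest is closed.
; OpenChest locks the open state, starts the lid timeline, then unbinds from the player and hides the prompt.
; The timeline derives lid rotation from normalized playback position instead of a curve track.
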(event OnComponentBeginOverlap(Box)
  (params (OverlappedComponent :type Primitive%20Component%20Object%20Reference) (OtherActor :type Actor%20Object%20Reference) (OtherComp :type Primitive%20Component%20Object%20Reference) (OtherBodyIndex :type Integer) (bFromSweep :type Boolean) (SweepResult :type Hit%20Result%20Structure%20%28by%20ref%29))
  (if (not (Variables|Default|GetbIsOpen))
    (bind _asbp_third_person_character (Utilities|Casting|CastToBP_ThirdPersonCharacter OtherActor))
    (EventDispatchers|BindEventtoOnInteract _asbp_third_person_character (EventDispatchers|CreateEvent :!event Custom|OpenChest))
    (CallFunction|Highlight)))

(event OnComponentEndOverlap(Box)
  (params (OverlappedComponent :type Primitive%20Component%20Object%20Reference) (OtherActor :type Actor%20Object%20Reference) (OtherComp :type Primitive%20Component%20Object%20Reference) (OtherBodyIndex :type Integer))
  (if (not (Variables|Default|GetbIsOpen))
    (bind _asbp_third_person_character (Utilities|Casting|CastToBP_ThirdPersonCharacter OtherActor))
    (EventDispatchers|UnbindEventfromOnInteract _asbp_third_person_character (EventDispatchers|CreateEvent :!event Custom|OpenChest))
    (CallFunction|Unhighlight)))

(event Custom|OpenChest
  (if (not (Variables|Default|GetbIsOpen))
    (Variables|Default|SetbIsOpen true)
    (Components|Timeline|PlayfromStart (Variables|Default|GetChestAnimation))
    (Audio|PlaySound2D "/Engine/VREditor/Sounds/VR_close.VR_close" 1.0 1.0 0.0 0 0)
    (Niagara|SpawnSystematLocation "/Niagara/DefaultAssets/Templates/Systems/AttributeReaderTrails.AttributeReaderTrails" (Transformation|GetWorldLocation (Variables|Default|GetVFXOrigin)) "0, 0, 0" "1.000000,1.000000,1.000000" true true "AutoRelease")
    (bind _asbp_third_person_character (Utilities|Casting|CastToBP_ThirdPersonCharacter (Game|GetPlayerCharacter 0)))
    (EventDispatchers|UnbindEventfromOnInteract _asbp_third_person_character (EventDispatchers|CreateEvent :!event Custom|OpenChest))
    (CallFunction|Unhighlight)))

(event EventBeginPlay
  (CallFunction|Unhighlight))

(fn ConstructionScript)

(fn Highlight
  (Rendering|SetVisibility (Variables|Default|GetTextRender) true false))

(fn Unhighlight
  (Rendering|SetVisibility (Variables|Default|GetTextRender) false false))